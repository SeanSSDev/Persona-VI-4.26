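; Volumetric clouds actor that renders the clouds' shadow into render targets every tick.
; On BeginPlay it stores the mesh's cloud material instance and creates a dynamic shadow material.
; Each update copies cloud shape, noise and texture parameters plus actor position and scale into that material, draws it to RT_Shadows, then draws a blur material into RT_Shadows_Blur.
; RenderShadows_EDITOR repeats this, creating the material first and using M_ShadowBlur instead of MI_ShadowBlur.
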(event EventBeginPlay
  (CallFunction|CreateMID))

(event Collision|EventActorBeginOverlap
  (params (OtherActor :type Actor%20Object%20Reference)))

(event EventTick
  (params (DeltaSeconds :type Float%20%28single-precision%29))
  (CallFunction|RenderShadows))

(fn ConstructionScript)

(fn RenderShadows
  (bind _returnvalue (Transformation|GetActorScale3D))
  (bind _returnvalue_2 (Transformation|GetActorLocation))
  (bind (_x _y _z) (Math|Vector|BreakVector _returnvalue_2))
  (bind (_x_2 _y_2 _z_2) (Math|Vector|BreakVector _returnvalue))
  (Utilities|ReadWriteMaterialFloat (Variables|Default|GetCloudsMI) (Variables|Default|GetShadowMID) "WeatherMapSzie"
    (:Out
      (Utilities|ReadWriteMaterialFloat (Variables|Default|GetCloudsMI) (Variables|Default|GetShadowMID) "Coverage"
        (:Out
          (Utilities|ReadWriteMaterialFloat (Variables|Default|GetCloudsMI) (Variables|Default|GetShadowMID) "WeatherMapOffsetX"
            (:Out
              (Utilities|ReadWriteMaterialFloat (Variables|Default|GetCloudsMI) (Variables|Default|GetShadowMID) "WeatherMapOffsetY"
                (:Out
                  (Utilities|ReadWriteMaterialFloat (Variables|Default|GetCloudsMI) (Variables|Default|GetShadowMID) "BaseNoiseSize"
                    (:Out
                      (Utilities|ReadWriteMaterialFloat (Variables|Default|GetCloudsMI) (Variables|Default|GetShadowMID) "DetailNoiseSize"
                        (:Out
                          (Utilities|ReadWriteMaterialFloat (Variables|Default|GetCloudsMI) (Variables|Default|GetShadowMID) "NoiseOffsetX"
                            (:Out
                              (Utilities|ReadWriteMaterialFloat (Variables|Default|GetCloudsMI) (Variables|Default|GetShadowMID) "NoiseOffsetY"
                                (:Out
                                  (Utilities|ReadWriteMaterialFloat (Variables|Default|GetCloudsMI) (Variables|Default|GetShadowMID) "NoiseOffsetZ"
                                    (:Out
                                      (Utilities|ReadWriteMaterialFloat (Variables|Default|GetCloudsMI) (Variables|Default|GetShadowMID) "DetailNoiseOffsetScale"
                                        (:Out
                                          (Utilities|ReadWriteMaterialFloat (Variables|Default|GetCloudsMI) (Variables|Default|GetShadowMID) "DistortionMapSize"
                                            (:Out
                                              (Utilities|ReadWriteMaterialFloat (Variables|Default|GetCloudsMI) (Variables|Default|GetShadowMID) "DistortionIntensity"
                                                (:Out
                                                  (Utilities|ReadWriteMaterialFloat (Variables|Default|GetCloudsMI) (Variables|Default|GetShadowMID) "CloudsDensity"
                                                    (:Out
                                                      (Utilities|ReadWriteMaterialTexture (Variables|Default|GetCloudsMI) (Variables|Default|GetShadowMID) "WeatherMap"
                                                        (:Out
                                                          (Utilities|ReadWriteMaterialTexture (Variables|Default|GetCloudsMI) (Variables|Default|GetShadowMID) "BaseNoise"
                                                            (:Out
                                                              (Utilities|ReadWriteMaterialTexture (Variables|Default|GetCloudsMI) (Variables|Default|GetShadowMID) "DetailNoise"
                                                                (:Out
                                                                  (Utilities|ReadWriteMaterialTexture (Variables|Default|GetCloudsMI) (Variables|Default|GetShadowMID) "DistortionMap"
                                                                    (:Out
                                                                      (Rendering|Material|SetScalarParameterValue (Variables|Default|GetShadowMID) "ActorPosX" _x :!class /Script/Engine.MaterialInstanceDynamic)
                                                                      (Rendering|Material|SetScalarParameterValue (Variables|Default|GetShadowMID) "ActorPosY" _y :!class /Script/Engine.MaterialInstanceDynamic)
                                                                      (Rendering|Material|SetScalarParameterValue (Variables|Default|GetShadowMID) "ActorPosZ" _z :!class /Script/Engine.MaterialInstanceDynamic)
                                                                      (Rendering|Material|SetScalarParameterValue (Variables|Default|GetShadowMID) "ActorScaleX" _x_2 :!class /Script/Engine.MaterialInstanceDynamic)
                                                                      (Rendering|Material|SetScalarParameterValue (Variables|Default|GetShadowMID) "ActorScaleY" _y_2 :!class /Script/Engine.MaterialInstanceDynamic)
                                                                      (Rendering|Material|SetScalarParameterValue (Variables|Default|GetShadowMID) "ActorScaleZ" _z_2 :!class /Script/Engine.MaterialInstanceDynamic)
                                                                      (Rendering|ClearRenderTarget2D "/Game/VolumetricClouds/Textures/RenderTargets/RT_Shadows.RT_Shadows")
                                                                      (bind (_canvas _size _context) (Rendering|BeginDrawCanvastoRenderTarget "/Game/VolumetricClouds/Textures/RenderTargets/RT_Shadows.RT_Shadows"))
                                                                      (Canvas|DrawMaterial :self _canvas :RenderMaterial (Variables|Default|GetShadowMID) :ScreenSize _size :CoordinateSize "(X=1.000000,Y=1.000000)" :PivotPoint "(X=0.500000,Y=0.500000)")
                                                                      (Rendering|EndDrawCanvastoRenderTarget _context)
                                                                      (Rendering|ClearRenderTarget2D "/Game/VolumetricClouds/Textures/RenderTargets/RT_Shadows_Blur.RT_Shadows_Blur")
                                                                      (bind (_canvas_2 _size_2 _context_2) (Rendering|BeginDrawCanvastoRenderTarget "/Game/VolumetricClouds/Textures/RenderTargets/RT_Shadows_Blur.RT_Shadows_Blur"))
                                                                      (Canvas|DrawMaterial :self _canvas_2 :RenderMaterial "/Game/VolumetricClouds/Materials/GroundShadows/MI_ShadowBlur.MI_ShadowBlur" :ScreenSize _size_2 :CoordinateSize "(X=1.000000,Y=1.000000)" :PivotPoint "(X=0.500000,Y=0.500000)")
                                                                      (Rendering|EndDrawCanvastoRenderTarget _context_2))))))))))))))))))))))))))))))))))))

(fn CreateMID
  (bind _asmaterial_instance_constant (Utilities|Casting|CastToMaterialInstanceConstant (Rendering|Material|GetMaterial (Variables|Debug|GetStaticMeshComponent) 0))
    (:then
      (Variables|Default|SetCloudsMI _asmaterial_instance_constant))
    (:CastFailed
      _))
  (bind _returnvalue (Rendering|Material|CreateDynamicMaterialInstance (Variables|Default|GetShadowMI) "None" "None" :!class /Script/Engine.KismetMaterialLibrary))
  (Variables|Default|SetShadowMID _returnvalue))

(fn RenderShadowsEDITOR
  (bind _returnvalue (Transformation|GetActorScale3D))
  (bind _returnvalue_2 (Transformation|GetActorLocation))
  (bind (_x _y _z) (Math|Vector|BreakVector _returnvalue_2))
  (bind (_x_2 _y_2 _z_2) (Math|Vector|BreakVector _returnvalue))
  (CallFunction|CreateMID)
  (Utilities|ReadWriteMaterialFloat (Variables|Default|GetCloudsMI) (Variables|Default|GetShadowMID) "WeatherMapSzie"
    (:Out
      (Utilities|ReadWriteMaterialFloat (Variables|Default|GetCloudsMI) (Variables|Default|GetShadowMID) "Coverage"
        (:Out
          (Utilities|ReadWriteMaterialFloat (Variables|Default|GetCloudsMI) (Variables|Default|GetShadowMID) "WeatherMapOffsetX"
            (:Out
              (Utilities|ReadWriteMaterialFloat (Variables|Default|GetCloudsMI) (Variables|Default|GetShadowMID) "WeatherMapOffsetY"
                (:Out
                  (Utilities|ReadWriteMaterialFloat (Variables|Default|GetCloudsMI) (Variables|Default|GetShadowMID) "BaseNoiseSize"
                    (:Out
                      (Utilities|ReadWriteMaterialFloat (Variables|Default|GetCloudsMI) (Variables|Default|GetShadowMID) "DetailNoiseSize"
                        (:Out
                          (Utilities|ReadWriteMaterialFloat (Variables|Default|GetCloudsMI) (Variables|Default|GetShadowMID) "NoiseOffsetX"
                            (:Out
                              (Utilities|ReadWriteMaterialFloat (Variables|Default|GetCloudsMI) (Variables|Default|GetShadowMID) "NoiseOffsetY"
                                (:Out
                                  (Utilities|ReadWriteMaterialFloat (Variables|Default|GetCloudsMI) (Variables|Default|GetShadowMID) "NoiseOffsetZ"
                                    (:Out
                                      (Utilities|ReadWriteMaterialFloat (Variables|Default|GetCloudsMI) (Variables|Default|GetShadowMID) "DetailNoiseOffsetScale"
                                        (:Out
                                          (Utilities|ReadWriteMaterialFloat (Variables|Default|GetCloudsMI) (Variables|Default|GetShadowMID) "DistortionMapSize"
                                            (:Out
                                              (Utilities|ReadWriteMaterialFloat (Variables|Default|GetCloudsMI) (Variables|Default|GetShadowMID) "DistortionIntensity"
                                                (:Out
                                                  (Utilities|ReadWriteMaterialFloat (Variables|Default|GetCloudsMI) (Variables|Default|GetShadowMID) "CloudsDensity"
                                                    (:Out
                                                      (Utilities|ReadWriteMaterialTexture (Variables|Default|GetCloudsMI) (Variables|Default|GetShadowMID) "WeatherMap"
                                                        (:Out
                                                          (Utilities|ReadWriteMaterialTexture (Variables|Default|GetCloudsMI) (Variables|Default|GetShadowMID) "BaseNoise"
                                                            (:Out
                                                              (Utilities|ReadWriteMaterialTexture (Variables|Default|GetCloudsMI) (Variables|Default|GetShadowMID) "DetailNoise"
                                                                (:Out
                                                                  (Utilities|ReadWriteMaterialTexture (Variables|Default|GetCloudsMI) (Variables|Default|GetShadowMID) "DistortionMap"
                                                                    (:Out
                                                                      (Rendering|Material|SetScalarParameterValue (Variables|Default|GetShadowMID) "ActorPosX" _x :!class /Script/Engine.MaterialInstanceDynamic)
                                                                      (Rendering|Material|SetScalarParameterValue (Variables|Default|GetShadowMID) "ActorPosY" _y :!class /Script/Engine.MaterialInstanceDynamic)
                                                                      (Rendering|Material|SetScalarParameterValue (Variables|Default|GetShadowMID) "ActorPosZ" _z :!class /Script/Engine.MaterialInstanceDynamic)
                                                                      (Rendering|Material|SetScalarParameterValue (Variables|Default|GetShadowMID) "ActorScaleX" _x_2 :!class /Script/Engine.MaterialInstanceDynamic)
                                                                      (Rendering|Material|SetScalarParameterValue (Variables|Default|GetShadowMID) "ActorScaleY" _y_2 :!class /Script/Engine.MaterialInstanceDynamic)
                                                                      (Rendering|Material|SetScalarParameterValue (Variables|Default|GetShadowMID) "ActorScaleZ" _z_2 :!class /Script/Engine.MaterialInstanceDynamic)
                                                                      (Rendering|ClearRenderTarget2D "/Game/VolumetricClouds/Textures/RenderTargets/RT_Shadows.RT_Shadows")
                                                                      (bind (_canvas _size _context) (Rendering|BeginDrawCanvastoRenderTarget "/Game/VolumetricClouds/Textures/RenderTargets/RT_Shadows.RT_Shadows"))
                                                                      (Canvas|DrawMaterial :self _canvas :RenderMaterial (Variables|Default|GetShadowMID) :ScreenSize _size :CoordinateSize "(X=1.000000,Y=1.000000)" :PivotPoint "(X=0.500000,Y=0.500000)")
                                                                      (Rendering|EndDrawCanvastoRenderTarget _context)
                                                                      (Rendering|ClearRenderTarget2D "/Game/VolumetricClouds/Textures/RenderTargets/RT_Shadows_Blur.RT_Shadows_Blur")
                                                                      (bind (_canvas_2 _size_2 _context_2) (Rendering|BeginDrawCanvastoRenderTarget "/Game/VolumetricClouds/Textures/RenderTargets/RT_Shadows_Blur.RT_Shadows_Blur"))
                                                                      (Canvas|DrawMaterial :self _canvas_2 :RenderMaterial "/Game/VolumetricClouds/Materials/GroundShadows/Base/M_ShadowBlur.M_ShadowBlur" :ScreenSize _size_2 :CoordinateSize "(X=1.000000,Y=1.000000)" :PivotPoint "(X=0.500000,Y=0.500000)")
                                                                      (Rendering|EndDrawCanvastoRenderTarget _context_2))))))))))))))))))))))))))))))))))))